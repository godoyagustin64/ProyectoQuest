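; Quest component that tracks a list of runtime quests and their objective progress.
; On BeginPlay it binds to gameplay objective events from BP_QuestGameState, matching type and target ID against objectives of active, uncompleted quests.
; AddQuest rejects duplicate IDs, while progress updates clamp to the required amount and rebuild the quest structs in the array.
; Each update triggers a completion check, with events for quest start, progress and completion.
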(event `self.ReceiveBeginPlay`
  (bind _asbp_quest_game_state (cast `/Game/QuestSystem/BP_QuestGameState` (`GameplayStatics.GetGameState`)))
  (add `/Game/QuestSystem/BP_QuestGameState.OnGameplayObjectiveEvent` _asbp_quest_game_state (delegate `HandleGameplayObjective`)))

(event `HandleGameplayObjective`
  (params (ObjectiveType :type "/Game/QuestSystem/EQuestObjectiveType Enum" :default "NewEnumerator0") (TargetID :type Name) (Amount :type Integer))
  (for (_array_element _array_index) (`self.ActiveQuests`)
    (bind (_questid _questdefinition _objectives _isactive _iscompleted) (break `/Game/QuestSystem/ST_QuestRuntime` _array_element))
    (if (and _isactive (not _iscompleted))
      (for (_array_element_2 _array_index_2) _objectives
        (bind (_objectiveid _objectivetype _targetid) (break `/Game/QuestSystem/ST_QuestObjective` _array_element_2))
        (if (and (`|EnumEquality` _objectivetype ObjectiveType) (== _targetid TargetID))
          (`self.UpdateObjectiveProgress` _array_index _array_index_2 Amount))))))

(fn `AddQuest`
  (params (QuestDefinition :type "/Game/QuestSystem/PDA_QuestDefinition Object Reference"))
  (bind _found (`self.FindQuestByID` (`/Game/QuestSystem/PDA_QuestDefinition.QuestID` QuestDefinition)))
  (if (not _found)
    (bind _returnvalue (`KismetArrayLibrary.Array_Add` (`self.ActiveQuests`) (make `/Game/QuestSystem/ST_QuestRuntime` (`/Game/QuestSystem/PDA_QuestDefinition.QuestID` QuestDefinition) QuestDefinition (`/Game/QuestSystem/PDA_QuestDefinition.Objectives` QuestDefinition) true)))
    (`self.OnQuestStarted` (`|GetArrayItem` (`self.ActiveQuests`) _returnvalue))))

(fn `CheckQuestCompleted`
  (params (QuestIndex :type Integer))
  (locals (AllObjectivesCompleted :type Boolean :default true))
  (bind (_questid _questdefinition _objectives) (break `/Game/QuestSystem/ST_QuestRuntime` (`|GetArrayItem` (`self.ActiveQuests`) QuestIndex)))
  (for (_array_element _array_index) _objectives
    (bind (_objectiveid _objectivetype _targetid _requiredamount _currentamount) (break `/Game/QuestSystem/ST_QuestObjective` _array_element))
    (if (not (>= _currentamount _requiredamount))
      (set `local.AllObjectivesCompleted` false)))
  (if (`local.AllObjectivesCompleted`)
    (`KismetArrayLibrary.Array_Set` (`self.ActiveQuests`) _array_index (make `/Game/QuestSystem/ST_QuestRuntime` _questid _questdefinition _objectives false true))
    (`self.OnQuestCompleted` (`|GetArrayItem` (`self.ActiveQuests`) (`local.QuestIndex`)))))

(fn `FindQuestByID`
  (params (QuestID :type Name))
  (returns (Found :type Boolean) (QuestData :type "/Game/QuestSystem/ST_QuestRuntime Structure") (QuestIndex :type Integer))
  (locals (FoundResult :type Boolean) (QuestDataResult :type "/Game/QuestSystem/ST_QuestRuntime Structure") (QuestIndexResult :type Integer))
  (set `local.FoundResult` false)
  (set `local.QuestIndexResult` -1)
  (for (_array_element _array_index) (`self.ActiveQuests`)
    (if (== (`.QuestID_2_6BCA7E8340C284B697271FB6DF723B98` (break `/Game/QuestSystem/ST_QuestRuntime` _array_element)) QuestID)
      (set `local.FoundResult` true)
      (set `local.QuestDataResult` _array_element)
      (set `local.QuestIndexResult` _array_index)
      (break)))
  (return (`local.FoundResult`) (`local.QuestDataResult`) (`local.QuestIndexResult`)))

(fn `UpdateObjectiveProgress`
  (params (QuestIndex :type Integer) (ObjectiveIndex :type Integer) (Amount :type Integer))
  (locals (UpdatedObjectives :type "Array of /Game/QuestSystem/ST_QuestObjective Structure"))
  (bind (_questid _questdefinition _objectives _isactive _iscompleted) (break `/Game/QuestSystem/ST_QuestRuntime` (`|GetArrayItem` (`self.ActiveQuests`) QuestIndex)))
  (bind _output_get (set `local.UpdatedObjectives` _objectives))
  (bind (_objectiveid _objectivetype _targetid _requiredamount _currentamount) (break `/Game/QuestSystem/ST_QuestObjective` (`|GetArrayItem` _output_get ObjectiveIndex)))
  (`KismetArrayLibrary.Array_Set` (`local.UpdatedObjectives`) (`local.ObjectiveIndex`) (make `/Game/QuestSystem/ST_QuestObjective` _objectiveid _objectivetype _targetid _requiredamount (`KismetMathLibrary.Min` (+ _currentamount Amount) _requiredamount)))
  (`KismetArrayLibrary.Array_Set` (`self.ActiveQuests`) (`local.QuestIndex`) (make `/Game/QuestSystem/ST_QuestRuntime` _questid _questdefinition (`local.UpdatedObjectives`) _isactive _iscompleted))
  (`self.OnQuestProgressChanged` (`|GetArrayItem` (`self.ActiveQuests`)))
  (`self.CheckQuestCompleted` (`local.QuestIndex`)))